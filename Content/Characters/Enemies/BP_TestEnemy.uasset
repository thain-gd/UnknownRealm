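; BP_TestEnemy is a test enemy that walks toward the village when play begins.
; On BeginPlay it finds actors tagged Village and, if the first is valid, orders its AI controller to move to it.
; Debug prints show the move request result and the name of any actor that begins overlapping it.
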(event EventBeginPlay
  (bind _outactors (Actor|GetAllActorswithTag "Village"))
  (Utilities|IsValid (Utilities|Array|Get(acopy) _outactors)
    (:Is%20Valid
      (bind _returnvalue (AI|Navigation|MovetoActor (AI|GetAIController self) (Utilities|Array|Get(acopy) _outactors) -1.0 true true true 0))
      (Development|PrintString (Utilities|String|EnumtoString _returnvalue) true true "(R=0.000000,G=0.660000,B=1.000000,A=1.000000)" 0.0))))

(event Collision|EventActorBeginOverlap
  (params (OtherActor :type Actor%20Object%20Reference))
  (Development|PrintString (Utilities|GetObjectName OtherActor) true true "(R=0.000000,G=0.660000,B=1.000000,A=1.000000)" 1e+01))

(fn ConstructionScript)