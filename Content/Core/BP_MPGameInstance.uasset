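; Multiplayer game instance that hosts and joins online sessions and handles connection errors.
; Hosting creates a session with optional LAN and opens DemoMap as a listen server, while joining uses a selected search result, both behind a loading screen.
; Session failures, travel errors and server-flagged network errors become messages for DisplayErrorDialog.
; On a successful transition to Startup, it destroys the session and shows a reused error widget with UI-only input.
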(event Custom|JoinGame
  (params (GameToJoin :type Blueprint%20Session%20Result%20Structure))
  ;[1 1 1] Join a selected game room
  (Class|MPGameInstance|ShowLoadingScreen)
  (|JoinSession (Game|GetPlayerController 0) GameToJoin
    (:OnFailure
      (CallFunction|DisplayErrorDialog "FAILED TO JOIN"))))

(event Custom|DestroySession
  (|DestroySession (Game|GetPlayerController 0)))

(event EventHostGame
  ;[1 1 1] Host a game
  (Class|MPGameInstance|ShowLoadingScreen)
  (|Session (Game|GetPlayerController 0) 4 (Variables|Default|GetbEnableLAN)
    (:OnSuccess
      (Game|OpenLevel(byName) "DemoMap" true "listen"))
    (:OnFailure
      (CallFunction|DisplayErrorDialog "FAILED! NO SESSION CREATED"))))

(event EventHandleNetworkError
  (params (FailureType :type ENetworkFailure%20Enum :default "NetDriverAlreadyExists") (bIsServer :type Boolean))
  ;[1 1 1] Error Handlers
  (if bIsServer
    (CallFunction|DisplayErrorDialog (CallFunction|NetErrortoString FailureType))))

(event EventHandleTravelError
  (params (FailureType :type ETravelFailure%20Enum :default "NoLevel"))
  ;[1 1 1] Error Handlers
  (CallFunction|DisplayErrorDialog (CallFunction|TravelErrortoString FailureType)))

(fn DisplayErrorDialog
  (params (ErrorMessage :type String))
  (bind _returnvalue (Class|MPGameInstance|TransitiontoState "Startup"))
  (if _returnvalue
    (CallFunction|DestroySession)
    (Utilities|IsValid (Variables|Default|GetErrorScreen)
      (:Is%20Valid
        _)
      (:Is%20Not%20Valid
        (bind _returnvalue_2 (UserInterface|CreateWidget "/Game/UI/UI_ErrorScreen.UI_ErrorScreen_C"))
        (bind _output_get (Variables|Default|SetErrorScreen _returnvalue_2))
        (bind _asui_error_screen (Utilities|Casting|CastToUI_ErrorScreen _output_get))))
    (Default|SetMessage _asui_error_screen ErrorMessage)
    (UserInterface|Viewport|AddtoViewport (Variables|Default|GetErrorScreen) 0)
    (Input|SetInputModeUIOnly (Game|GetPlayerController 0) (Variables|Default|GetErrorScreen) "DoNotLock")))

(fn NetErrortoString
  (params (InError :type ENetworkFailure%20Enum :default "NetDriverAlreadyExists"))
  (switch Utilities|FlowControl|Switch|SwitchonENetworkFailure InError
    (:NetDriverAlreadyExists
      (LocalVariables|SetErrorString "ERROR: CONNECTION LOST" :!label _label))
    (:NetDriverCreateFailure
      (goto _label))
    (:NetDriverListenFailure
      (goto _label))
    (:ConnectionLost
      (goto _label))
    (:ConnectionTimeout
      (LocalVariables|SetErrorString "ERROR: CONNECTION TIMED OUT"))
    (:FailureReceived
      (goto _label))
    (:OutdatedClient
      (goto _label))
    (:OutdatedServer
      (goto _label))
    (:PendingConnectionFailure
      (goto _label)))
  (return (LocalVariables|GetErrorString)))

(fn TravelErrortoString
  (params (InError :type ETravelFailure%20Enum :default "NoLevel"))
  (return (Utilities|String|Append "ERROR: TRAVEL FAILURE " (Utilities|String|EnumtoString InError))))