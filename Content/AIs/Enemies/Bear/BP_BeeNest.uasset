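; Bee nest projectile in the Bear enemy's folder that damages the player on contact.
; OnThrown launches it along its owner's forward vector through ProjectileMovement, with low speed and reduced gravity.
; When its static mesh overlaps an actor tagged Player, it prints a debug string, applies damage and destroys itself.
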(event OnComponentBeginOverlap(StaticMesh)
  (params (OverlappedComponent :type Primitive%20Component%20Object%20Reference) (OtherActor :type Actor%20Object%20Reference) (OtherComp :type Primitive%20Component%20Object%20Reference) (OtherBodyIndex :type Integer) (bFromSweep :type Boolean) (SweepResult :type Hit%20Result%20Structure%20%28by%20ref%29))
  (if (Actor|ActorHasTag OtherActor "Player")
    (Development|PrintString "Bloop!!!")
    (Game|Damage|ApplyDamage OtherActor 15.0 0 0 "/Script/UnknownRealm.BaseDamageType")
    (Actor|DestroyActor)))

(event Custom|OnThrown
  (bind _projectilemovement (Variables|Default|GetProjectileMovement))
  (Variables|/Script/Engine.MovementComponent|SetVelocity _projectilemovement (* (Transformation|GetActorForwardVector (Components|GetOwner)) 1e+02))
  (Variables|/Script/Engine.ProjectileMovementComponent|SetProjectileGravityScale _projectilemovement 0.2))

(fn ConstructionScript)