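; BP_Enemy is an enemy that walks to the village and damages it on contact.
; On BeginPlay the server finds the first actor tagged "Village" and has the AI controller move to it, printing the request result.
; When its Box component overlaps a Village-tagged actor, the server applies fixed damage to that actor.
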(event OnComponentBeginOverlap(Box)
  (params (OverlappedComponent :type Primitive%20Component%20Object%20Reference) (OtherActor :type Actor%20Object%20Reference) (OtherComp :type Primitive%20Component%20Object%20Reference) (OtherBodyIndex :type Integer) (bFromSweep :type Boolean) (SweepResult :type Hit%20Result%20Structure%20%28by%20ref%29))
  (Networking|SwitchHasAuthority
    (:Authority
      (if (Actor|ActorHasTag OtherActor "Village")
        (Game|Damage|ApplyDamage OtherActor 3e+01 0 0)))))

(event EventBeginPlay
  (Networking|SwitchHasAuthority
    (:Authority
      (bind _outactors (Actor|GetAllActorswithTag "Village"))
      (Utilities|IsValid (Utilities|Array|Get(acopy) _outactors)
        (:Is%20Valid
          (bind _returnvalue (AI|Navigation|MovetoActor (AI|GetAIController self) (Utilities|Array|Get(acopy) _outactors) -1.0 true true true 0))
          (Development|PrintString (Utilities|String|EnumtoString _returnvalue) true true "(R=0.000000,G=0.660000,B=1.000000,A=1.000000)" 0.0))))))

(event Collision|EventActorBeginOverlap
  (params (OtherActor :type Actor%20Object%20Reference)))

(fn ConstructionScript)