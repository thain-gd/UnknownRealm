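; BP_BuildingManager tracks the Village actors in the level and picks which one an enemy should target.
; BeginPlay caches every Village actor in the Tents array with GetAllActorsOfClass.
; GetClosestTarget loops over that array and returns the Village closest to the given enemy that still has a targetable location available, comparing squared distances.
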(event EventBeginPlay
  (bind _outactors (Actor|GetAllActorsOfClass "/Script/UnknownRealm.Village"))
  (Variables|Default|SetTents _outactors))

(fn ConstructionScript)

(fn GetClosestTarget
  (params (Enemy :type AI%20Char%20Object%20Reference))
  (for _array_element (Variables|Default|GetTents)
    (if (and (< (Transformation|GetSquaredDistanceTo Enemy _array_element) (LocalVariables|GetClosestDistanceSquared)) (Class|Village|IsAnyTargetableLocationAvailable _array_element))
      (LocalVariables|SetClosestDistanceSquared (Transformation|GetSquaredDistanceTo Enemy _array_element))
      (LocalVariables|SetClosestTarget _array_element)))
  (return (LocalVariables|GetClosestTarget)))